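; Pushable statue that slides a fixed distance along a rounded axis when the player walks into it head-on.
; On Hit, a line trace confirms the player faces the statue and a box trace checks the path is clear.
; Push disables player movement, attaches the player, drives the statue by timeline and flags ABP_Manny as interacting, then detaches and restores walking.
; A separate Speed/Direction graph offers interpolated mesh movement but is not called here.
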(event `self.ReceiveHit`
  (params (MyComp :type "PrimitiveComponent Object Reference") (Other :type "Actor Object Reference") (OtherComp :type "PrimitiveComponent Object Reference") (bSelfMoved :type Boolean) (HitLocation :type "Vector Structure") (HitNormal :type "Vector Structure") (NormalImpulse :type "Vector Structure") (Hit :type "HitResult Structure (by ref)"))
  (bind _returnvalue (`GameplayStatics.GetPlayerCharacter` 0))
  (bind _returnvalue_2 (`self.GetActorForwardVector` Other))
  (`KismetSystemLibrary.PrintString` (`KismetSystemLibrary.GetDisplayName` Other))
  (if (== (`GameplayStatics.GetPlayerCharacter` 0) Other)
    (if (> (`KismetMathLibrary.Dot_VectorVector` HitNormal _returnvalue_2) 0.93)
      (set `self.PushableDirection` (`KismetMathLibrary.MakeVector` (`KismetMathLibrary.Conv_IntToDouble` (`KismetMathLibrary.Round` (.x _returnvalue_2))) (`KismetMathLibrary.Conv_IntToDouble` (`KismetMathLibrary.Round` (.y _returnvalue_2))) (`KismetMathLibrary.Conv_IntToDouble` (`KismetMathLibrary.Round` (.z _returnvalue_2)))))
      (bind _can_push (`self.CanPush`))
      (if _can_push
        (`CharacterMovementComponent.DisableMovement` (`Character.CharacterMovement` _returnvalue))
        (`self.K2_AttachToActor` _returnvalue self "None" "KeepWorld" "KeepWorld" "KeepWorld" true)
        (`self.Push`)))))

(event `Push`
  (set `self.Current Location` (`self.K2_GetActorLocation`))
  (bind (_direction _position) (`Timeline|MoveBack` :!via `PlayFromStart`)
    (:`Update`
      (set `/Game/Characters/Mannequins/Animations/ABP_Manny.Is Interacting Box?` true (`self.As ABP Manny`))
      (`self.K2_SetActorRelativeLocation` (+ (`self.Current Location`) (* _position (`self.PushableDirection`) (`self.Travel Distance`)))))
    (:`Finished`
      (`self.Stop Pushing`))))

(event `self.ReceiveBeginPlay`
  (`KismetSystemLibrary.DelayUntilNextTick`)
  (bind _asbp_third_person_feli (cast `/Game/ThirdPerson/Blueprints/BP_ThirdPersonFeli` (`GameplayStatics.GetPlayerCharacter` 0)))
  (set `self.Char REF` _asbp_third_person_feli)
  (bind _asabp_manny (cast `/Game/Characters/Mannequins/Animations/ABP_Manny` (`SkeletalMeshComponent.GetAnimInstance` (`Character.Mesh` (`self.Char REF`)))))
  (set `self.As ABP Manny` _asabp_manny))

(event `Stop Pushing`
  (bind _returnvalue (`GameplayStatics.GetPlayerCharacter` 0))
  (`CharacterMovementComponent.SetMovementMode` (`Character.CharacterMovement` _returnvalue) "MOVE_Walking" 0)
  (`self.K2_DetachFromActor` _returnvalue "KeepWorld" "KeepWorld" "KeepWorld"))

(fn `CanPush`
  (returns (`Can Push` :type Boolean))
  (bind _returnvalue (`GameplayStatics.GetPlayerCharacter` 0))
  (bind _returnvalue_2 (`self.K2_GetActorLocation`))
  (bind _returnvalue_3 (`self.K2_GetActorLocation` _returnvalue))
  (bind (_returnvalue_origin _returnvalue_boxextent) (`KismetMathLibrary.BreakBoxSphereBounds` (`StaticMesh.GetBounds` (`StaticMeshComponent.StaticMesh` (`self.SM_Statue`)))))
  (bind (_outhit _returnvalue_4) (`KismetSystemLibrary.LineTraceSingle` _returnvalue_3 (+ _returnvalue_3 (* (`self.GetActorForwardVector` _returnvalue) 200.0)) "TraceTypeQuery1" false (`|MakeArray` _returnvalue :!type "Actor Object Reference") "None" false))
  (if _returnvalue_4
    (if (== (`.HitActor` (`GameplayStatics.BreakHitResult` _outhit)) self)
      (bind (_outhit_2 _returnvalue_5) (`KismetSystemLibrary.BoxTraceSingle` (+ _returnvalue_2 (0.0 0.0 100.0)) (+ _returnvalue_2 (* (`self.PushableDirection`) (`self.Travel Distance`) (0.9 0.9 0.9)) (0.0 0.0 100.0)) (* _returnvalue_boxextent (`SceneComponent.RelativeScale3D` (`self.SM_Statue`))) (struct) "TraceTypeQuery1" false (`|MakeArray` _returnvalue :!type "Actor Object Reference") "ForDuration"))
      (`KismetSystemLibrary.PrintString` (`KismetSystemLibrary.GetDisplayName` (`.HitActor` (`GameplayStatics.BreakHitResult` _outhit_2))))
      (return (not _returnvalue_5))
      (else
        (return false)))
    (else
      (return false))))

(fn `UserConstructionScript`)