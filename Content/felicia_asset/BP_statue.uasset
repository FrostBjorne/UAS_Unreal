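; BP_statue is a statue actor that the BP_ThirdPersonFeli player can push around while interacting.
; Overlapping the FWD component enables interaction; leaving it clears interaction and resets walk speed.
; Tick reads the character's movement axes and calls SpeedDirection, which VInterps the mesh along its right or forward vector without sweeping.
; Forward and backward input both move it the same way; debug prints report state.
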(event `self.ReceiveBeginPlay`
  (`GameplayStatics.GetActorOfClass` "/Game/ThirdPerson/Blueprints/BP_ThirdPersonFeli.BP_ThirdPersonFeli_C")
  (`KismetSystemLibrary.DelayUntilNextTick`)
  (bind _asbp_third_person_feli (cast `/Game/ThirdPerson/Blueprints/BP_ThirdPersonFeli` (`GameplayStatics.GetPlayerCharacter` 0)))
  (set `self.Char REF` _asbp_third_person_feli))

(event `self.ReceiveTick`
  (params (DeltaSeconds :type "Float (single-precision)"))
  (bind _char_ref (`self.Char REF`))
  (bind _forward_bakcward_axis (`/Game/ThirdPerson/Blueprints/BP_ThirdPersonFeli.Forward Bakcward Axis` _char_ref))
  (bind _right_left_axis (`/Game/ThirdPerson/Blueprints/BP_ThirdPersonFeli.Right Left Axis` _char_ref))
  (bind _char_ref_2 (`self.Char REF`)
    (:`then`
      (if (`/Game/ThirdPerson/Blueprints/BP_ThirdPersonFeli.IsInteractingBox?` _char_ref_2)
        (if (`/Game/ThirdPerson/Blueprints/BP_ThirdPersonFeli.CanInteractBox?` _char_ref_2)
          (`|ExecutionSequence`
            (:`then_0`
              (if (== _forward_bakcward_axis 0.0)
                (`KismetSystemLibrary.PrintString` "Is not moving forward or backward" true true (struct :`R` 1.0 :`B` 0.018015 :`A` 1.0) 2.0 "423423")
                (elif (>= _forward_bakcward_axis 0.1)
                  (`KismetSystemLibrary.PrintString` "Is Moving Forward" true true (struct :`R` 1.0 :`B` 0.018015 :`A` 1.0) 2.0 "342342322")
                  (`self.Speed/Direction` true 34.0)
                  (else
                    (`KismetSystemLibrary.PrintString` "Is Moving Backward" true true (struct :`R` 1.0 :`B` 0.018015 :`A` 1.0) 2.0 "5333")
                    (`self.Speed/Direction` true 34.0)))))
            (:`then_1`
              (if (== _right_left_axis 0.0)
                (`KismetSystemLibrary.PrintString` "Is not moving forward or backward" true true (struct :`R` 1.0 :`B` 0.018015 :`A` 1.0) 2.0 "423423")
                (elif (>= _right_left_axis 0.1)
                  (`KismetSystemLibrary.PrintString` "Is Moving Right" true true (struct :`R` 1.0 :`B` 0.018015 :`A` 1.0) 2.0 "342342322")
                  (`self.Speed/Direction` false -31.0)
                  (else
                    (`KismetSystemLibrary.PrintString` "Is Moving Left" true true (struct :`R` 1.0 :`B` 0.018015 :`A` 1.0) 2.0 "5333")
                    (`self.Speed/Direction` false 31.0)))))))))
    (:`else`)))

(event `self.FWD.OnComponentBeginOverlap`
  (params (OverlappedComponent :type "PrimitiveComponent Object Reference") (OtherActor :type "Actor Object Reference") (OtherComp :type "PrimitiveComponent Object Reference") (OtherBodyIndex :type Integer) (bFromSweep :type Boolean) (SweepResult :type "HitResult Structure (by ref)"))
  (`KismetSystemLibrary.PrintString` "Character Can Interact" true true (struct :`G` 1.0 :`B` 0.031802 :`A` 1.0) 2.0 "432342")
  (set `/Game/ThirdPerson/Blueprints/BP_ThirdPersonFeli.CanInteractBox?` true (`self.Char REF`)))

(event `self.FWD.OnComponentEndOverlap`
  (params (OverlappedComponent :type "PrimitiveComponent Object Reference") (OtherActor :type "Actor Object Reference") (OtherComp :type "PrimitiveComponent Object Reference") (OtherBodyIndex :type Integer))
  (bind _char_ref (`self.Char REF`))
  (`KismetSystemLibrary.PrintString` "Character Cannot Interact" true true (struct :`R` 1.0 :`B` 0.229062 :`A` 1.0) 2.0 "3423423423")
  (set `/Game/ThirdPerson/Blueprints/BP_ThirdPersonFeli.CanInteractBox?` false _char_ref)
  (set `CharacterMovementComponent.MaxWalkSpeed` 230.0 (`Character.CharacterMovement` _char_ref))
  (set `/Game/ThirdPerson/Blueprints/BP_ThirdPersonFeli.IsInteractingBox?` false _char_ref))

(fn `UserConstructionScript`)