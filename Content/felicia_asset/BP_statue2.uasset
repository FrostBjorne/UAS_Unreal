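; Pushable statue that slides one travel distance along the player's rounded facing direction when the player hits it head-on.
; CanPush uses traces to verify facing, clear space, floor ahead and nothing on top, plus that the player isn't falling.
; Push attaches the immobilized player and runs the MoveBack timeline; StopPushing releases them, then calls Push again without rechecking.
; A separate Speed/Direction graph interpolates the mesh along its forward or right vector.
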(event `self.ReceiveHit`
  (params (MyComp :type "PrimitiveComponent Object Reference") (Other :type "Actor Object Reference") (OtherComp :type "PrimitiveComponent Object Reference") (bSelfMoved :type Boolean) (HitLocation :type "Vector Structure") (HitNormal :type "Vector Structure") (NormalImpulse :type "Vector Structure") (Hit :type "HitResult Structure (by ref)"))
  (bind _returnvalue (`GameplayStatics.GetPlayerCharacter` 0))
  (bind _returnvalue_2 (`self.GetActorForwardVector` Other))
  (`KismetSystemLibrary.PrintString` (`KismetSystemLibrary.GetDisplayName` Other))
  (if (== (`GameplayStatics.GetPlayerCharacter` 0) Other)
    (if (> (`KismetMathLibrary.Dot_VectorVector` HitNormal _returnvalue_2) 0.93)
      (set `self.PushableDirection` (`KismetMathLibrary.MakeVector` (`KismetMathLibrary.Conv_IntToDouble` (`KismetMathLibrary.Round` (.x _returnvalue_2))) (`KismetMathLibrary.Conv_IntToDouble` (`KismetMathLibrary.Round` (.y _returnvalue_2))) (`KismetMathLibrary.Conv_IntToDouble` (`KismetMathLibrary.Round` (.z _returnvalue_2)))))
      (bind _can_push (`self.CanPush`))
      (if _can_push
        (`CharacterMovementComponent.DisableMovement` (`Character.CharacterMovement` _returnvalue))
        (`self.K2_AttachToActor` _returnvalue self "None" "KeepWorld" "KeepWorld" "KeepWorld" true)
        (`self.Push`)))))

(event `Push`
  (set `self.Current Location` (`self.K2_GetActorLocation`))
  (bind (_direction _position) (`Timeline|MoveBack` :!via `PlayFromStart`)
    (:`Update`
      (`self.K2_SetActorRelativeLocation` (+ (`self.Current Location`) (* _position (`self.PushableDirection`) (`self.Travel Distance`)))))
    (:`Finished`
      (`self.Stop Pushing`))))

(event `Stop Pushing`
  (bind _returnvalue (`GameplayStatics.GetPlayerCharacter` 0))
  (`CharacterMovementComponent.SetMovementMode` (`Character.CharacterMovement` _returnvalue) "MOVE_Walking" 0)
  (`self.K2_DetachFromActor` _returnvalue "KeepWorld" "KeepWorld" "KeepWorld")
  (`self.Push`))

(fn `CanPush`
  (returns (`Can Push` :type Boolean))
  (locals (LocalCanPush :type Boolean :default true))
  (bind _returnvalue (`GameplayStatics.GetPlayerCharacter` 0))
  (bind _returnvalue_2 (`self.K2_GetActorLocation`))
  (bind _returnvalue_3 (`self.K2_GetActorLocation` _returnvalue))
  (bind _returnvalue_4 (+ (`self.K2_GetActorLocation`) (0.0 0.0 200.0)))
  (bind (_returnvalue_origin _returnvalue_boxextent) (`KismetMathLibrary.BreakBoxSphereBounds` (`StaticMesh.GetBounds` (`StaticMeshComponent.StaticMesh` (`self.SM_Statue`)))))
  (bind _returnvalue_5 (+ (`self.K2_GetActorLocation`) (* (`self.PushableDirection`) (`self.Travel Distance`) 1.5) (0.0 0.0 100.0)))
  (`|ExecutionSequence`
    (:`then_0`
      ; 1. Check Player is Facing Box
      (bind (_outhit _returnvalue_6) (`KismetSystemLibrary.LineTraceSingle` _returnvalue_3 (+ _returnvalue_3 (* (`self.GetActorForwardVector` _returnvalue) 200.0)) "TraceTypeQuery1" false (`|MakeArray` _returnvalue :!type "Actor Object Reference") "None" false))
      (if _returnvalue_6
        (if (not (== (`.HitActor` (`GameplayStatics.BreakHitResult` _outhit)) self))
          (set `local.LocalCanPush` false))
        (else
          (set `local.LocalCanPush` false))))
    (:`then_1`
      ; 2. Check if Box has room to move
      (bind (_outhit_2 _returnvalue_7) (`KismetSystemLibrary.BoxTraceSingle` :`Start` (+ _returnvalue_2 (0.0 0.0 100.0)) :`End` (+ _returnvalue_2 (* (`self.PushableDirection`) (`self.Travel Distance`) (0.9 0.9 0.9)) (0.0 0.0 100.0)) :`HalfSize` (* _returnvalue_boxextent (`SceneComponent.RelativeScale3D` (`self.SM_Statue`))) :`TraceChannel` "TraceTypeQuery1" :`DrawDebugType` "ForDuration"))
      (if (not (not _returnvalue_7))
        (set `local.LocalCanPush` false)))
    (:`then_2`
      ; 3. Check if space has flooor
      (bind (_outhit_3 _returnvalue_8) (`KismetSystemLibrary.LineTraceSingle` :`Start` _returnvalue_5 :`End` (+ _returnvalue_5 (0.0 0.0 -200.0)) :`TraceChannel` "TraceTypeQuery1" :`DrawDebugType` "ForDuration"))
      (if (not _returnvalue_8)
        (set `local.LocalCanPush` false)))
    (:`then_3`
      ; 4. Check if anything on top of the box
      (bind (_outhit_4 _returnvalue_9) (`KismetSystemLibrary.LineTraceSingle` _returnvalue_4 (+ _returnvalue_4 (0.0 0.0 200.0)) "TraceTypeQuery1"))
      (if _returnvalue_9
        (set `local.LocalCanPush` false)))
    (:`then_4`
      ; 5. Check if player not falling
      (if (`NavMovementComponent.IsFalling` (`Character.CharacterMovement` (`GameplayStatics.GetPlayerCharacter` 0)))
        (set `local.LocalCanPush` false)))
    (:`then_5`
      (return (`local.LocalCanPush`)))))

(fn `UserConstructionScript`)