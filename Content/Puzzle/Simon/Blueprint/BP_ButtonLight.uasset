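; One button of the Simon puzzle, with its own color, sound and index, that lights up when its note plays.
; On the player's turn, overlapping it enables input and briefly shows a highlight overlay, and pressing E reports its index to the Simon main actor.
; PlayNote and PlayError drive audio and a dynamic material's glow for a second, with the error flashing red before restoring the button's color and sound.
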(event `self.ReceiveBeginPlay`
  (`AudioComponent.SetSound` (`self.Audio`) (`self.Sound`)))

(event `/Game/Puzzle/Simon/Blueprint/BPI_Interact.OnInteract`
  (params (Actor :type "Actor Object Reference"))
  ;[1 1 1] -
  (if (`KismetSystemLibrary.DoesImplementInterface` Actor "/Game/Puzzle/Simon/Blueprint/BPI_Interact.BPI_Interact_C")
    _))

(event `Key|E`
  (params (Key :type "Key Structure"))
  (:`Pressed`
    (bind _simonmain_ref (`self.SimonMain_Ref`)
      (:`then`
        (if (`/Game/Puzzle/Simon/Blueprint/BP_SimonManager.IsPlayersTurn` _simonmain_ref)
          (`/Game/Puzzle/Simon/Blueprint/BP_SimonManager.PlayerPlayedNote` (`self.SimonMain_Ref`) (`self.Index`))))
      (:`else`))))

(event `PlayNote`
  (`AudioComponent.Play` (`self.Audio`) 0.0)
  (`MaterialInstanceDynamic.SetScalarParameterValue` (`self.Dyn Mat`) "Intensity" 2.5)
  (`KismetSystemLibrary.Delay` 1.0)
  (`AudioComponent.Stop` (`self.Audio`))
  (`MaterialInstanceDynamic.SetScalarParameterValue` (`self.Dyn Mat`) "Intensity" 0.0))

(event `self.ReceiveActorBeginOverlap`
  (params (OtherActor :type "Actor Object Reference"))
  (bind _simonmain_ref (`self.SimonMain_Ref`)
    (:`then`
      (if (`/Game/Puzzle/Simon/Blueprint/BP_SimonManager.IsPlayersTurn` _simonmain_ref)
        (`self.EnableInput` (`GameplayStatics.GetPlayerController` 0))
        (`MeshComponent.SetOverlayMaterial` (`self.Button`) "/Game/Puzzle/Simon/Material/M_Overlay.M_Overlay")
        (`KismetSystemLibrary.RetriggerableDelay` 2.0)
        (`MeshComponent.SetOverlayMaterial` (`self.Button`) null)))
    (:`else`)))

(event `self.ReceiveActorEndOverlap`
  (params (OtherActor :type "Actor Object Reference"))
  (`self.DisableInput` null)
  (`MeshComponent.SetOverlayMaterial` (`self.Button`) null))

(event `PlayError`
  (`AudioComponent.SetSound` (`self.Audio`) null)
  (`AudioComponent.Play` (`self.Audio`) 0.0)
  (`MaterialInstanceDynamic.SetVectorParameterValue` (`self.Dyn Mat`) "Base Color" (struct :`R` 1.0 :`G` 0.135026 :`B` 0.055345 :`A` 1.0))
  (`MaterialInstanceDynamic.SetScalarParameterValue` (`self.Dyn Mat`) "Intensity" 2.5)
  (`KismetSystemLibrary.Delay` 1.0)
  (`AudioComponent.Stop` (`self.Audio`))
  (`MaterialInstanceDynamic.SetScalarParameterValue` (`self.Dyn Mat`) "Intensity" 0.0)
  (`MaterialInstanceDynamic.SetVectorParameterValue` (`self.Dyn Mat`) "Base Color" (`self.Color`))
  (`AudioComponent.SetSound` (`self.Audio`) (`self.Sound`)))

(fn `UserConstructionScript`
  (bind _returnvalue (`PrimitiveComponent.CreateDynamicMaterialInstance` (`self.Button`) 0 null "None"))
  (bind _output_get (set `self.Dyn Mat` _returnvalue))
  (`MaterialInstanceDynamic.SetVectorParameterValue` _output_get "Base Color" (`self.Color`)))