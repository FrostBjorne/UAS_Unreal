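; BP_SimonManager runs a Simon-style memory puzzle that starts on box overlap and powers a door once the last level is beaten.
; Each level builds a random button sequence from LevelSettings, plays it with delayed recursive events, then checks the player's notes.
; A correct sequence advances the level, while a mistake plays errors and restarts from the first.
; The construction script caps note counts at the button count when duplicates are disallowed.
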(event `self.ReceiveBeginPlay`
  ;[1 1 1] Set Reference in Button
  (for _array_element (`self.Buttons`)
    (`/Engine/EditorBlueprintResources/StandardMacros.IsValid` _array_element
      (:`Is Valid`
        (set `/Game/Puzzle/Simon/Blueprint/BP_ButtonLight.SimonMain_Ref` self _array_element))
      (:`Is Not Valid`
        (`KismetSystemLibrary.PrintString` "Forgot to set up stand" true true (struct :`R` 0.978642 :`G` 1.0 :`A` 1.0))))))

(event `AddNote`
  (bind (_numberofnotes _timebetweennotes _canduplicatenotes) (break `/Game/Puzzle/Simon/Blueprint/SimonLevel_Struct` (`|GetArrayItem` (`self.LevelSettings`) (`self.CurrentLevel`))))
  ;[1 1 1] Create Random Sequence
  (if (> (`KismetArrayLibrary.Array_Length` (`self.Buttons`)) 0) :!label _label
    (if _canduplicatenotes
      (`KismetArrayLibrary.Array_Add` (`self.SimonSequences`) (`KismetMathLibrary.RandomIntegerInRange` 0 (`KismetArrayLibrary.Array_LastIndex` (`self.Buttons`))))
      (else
        (`KismetArrayLibrary.Array_AddUnique` (`self.SimonSequences`) (`KismetMathLibrary.RandomIntegerInRange` 0 (`KismetArrayLibrary.Array_LastIndex` (`self.Buttons`))))))
    (if (< (`KismetArrayLibrary.Array_Length` (`self.SimonSequences`)) _numberofnotes)
      (`KismetSystemLibrary.Delay` 0.0)
      (`self.AddNote`)
      (else
        (`KismetSystemLibrary.Delay` 1.0)
        (`self.PlaySimonSequence`)))))

(event `CreateSimonSequence`
  ;[1 1 1] Create Random Sequence
  (`KismetArrayLibrary.Array_Clear` (`self.SimonSequences`))
  (goto _label))

(event `self.Box.OnComponentBeginOverlap`
  (params (OverlappedComponent :type "PrimitiveComponent Object Reference") (OtherActor :type "Actor Object Reference") (OtherComp :type "PrimitiveComponent Object Reference") (OtherBodyIndex :type Integer) (bFromSweep :type Boolean) (SweepResult :type "HitResult Structure (by ref)"))
  ;[1 1 1] Overlap-StartLevel
  (if (and (not (`self.IsPlayersTurn`)) (not (`self.IsPlaying`)))
    (set `self.IsPlaying` true)
    (`self.StartLevel`)))

(event `StartLevel`
  ;[1 1 1] New Level
  (`KismetArrayLibrary.Array_Clear` (`self.PlayerSequences`))
  (set `self.CurrentNote` 0)
  (set `self.IsPlayersTurn` false)
  (`self.CreateSimonSequence`))

(event `PlaySimonSequence`
  (`/Game/Puzzle/Simon/Blueprint/BP_ButtonLight.PlayNote` (`|GetArrayItem` (`self.Buttons`) (`|GetArrayItem` (`self.SimonSequences`) (`self.CurrentNote`))))
  (`KismetSystemLibrary.Delay` (`.TimeBetweenNotes_7_7CD1A59840003E41C09A1CA04713A678` (break `/Game/Puzzle/Simon/Blueprint/SimonLevel_Struct` (`|GetArrayItem` (`self.LevelSettings`) (`self.CurrentLevel`)))))
  (`/Engine/EditorBlueprintResources/StandardMacros.IncrementInt` (`self.CurrentNote`)
    (:`  `
      (if (< (`self.CurrentNote`) (`KismetArrayLibrary.Array_Length` (`self.SimonSequences`)))
        (`self.PlaySimonSequence`)
        (else
          (set `self.IsPlayersTurn` true))))))

(event `PlayerPlayedNote`
  (params (Note :type Integer))
  (set `self.IsPlayersTurn` false)
  (bind _returnvalue (`KismetArrayLibrary.Array_Add` (`self.PlayerSequences`) Note))
  (if (== Note (`|GetArrayItem` (`self.SimonSequences`) _returnvalue))
    (`/Game/Puzzle/Simon/Blueprint/BP_ButtonLight.PlayNote` (`|GetArrayItem` (`self.Buttons`) Note))
    (if (>= (`KismetArrayLibrary.Array_Length` (`self.PlayerSequences`)) (`KismetArrayLibrary.Array_Length` (`self.SimonSequences`)))
      (if (< (`self.CurrentLevel`) (`KismetArrayLibrary.Array_LastIndex` (`self.LevelSettings`)))
        (`/Engine/EditorBlueprintResources/StandardMacros.IncrementInt` (`self.CurrentLevel`)
          (:`  `
            (`KismetSystemLibrary.Delay` 2.0)
            (`self.StartLevel`)))
        (else
          (`KismetSystemLibrary.PrintString` "Player Wins")
          (`/Engine/EditorBlueprintResources/StandardMacros.DoOnce` false
            (:`Completed`
              (bind _doortoopen (`self.DoorToOpen`)
                (:`then`
                  (message `/Game/Puzzle/Cable/BI_Power.PowerOn` _doortoopen))
                (:`else`))))))
      (else
        (set `self.IsPlayersTurn` true)))
    (else
      (for _array_element (`self.Buttons`)
        (`/Game/Puzzle/Simon/Blueprint/BP_ButtonLight.PlayError` _array_element))
      (`KismetSystemLibrary.Delay` 2.0)
      (set `self.CurrentLevel` 0)
      (`self.StartLevel`))))

(fn `UserConstructionScript`
  (bind _returnvalue (`KismetArrayLibrary.Array_Length` (`self.Buttons`)))
  (for (_array_element _array_index) (`self.LevelSettings`)
    (bind ((`NumberofNotes_5_3F03E0AD47F92225CE7220BB9826445C` _numberofnotes) (`CanDuplicateNotes_10_6A8BD7D4431A279C9586A7B2ABECFDE6` _canduplicatenotes)) (break `/Game/Puzzle/Simon/Blueprint/SimonLevel_Struct` _array_element))
    (if _canduplicatenotes
      _
      (elif (> _numberofnotes _returnvalue)
        (bind _structout (setmembers `/Game/Puzzle/Simon/Blueprint/SimonLevel_Struct` :`StructRef` _array_element :`NumberofNotes` _returnvalue))
        (`KismetArrayLibrary.Array_Set` (`self.LevelSettings`) _array_index _structout)))))