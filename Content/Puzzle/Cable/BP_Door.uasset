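; BP_Door is a puzzle door that swings open on the Poweron event and closed on PowerOff.
; Each event restarts its own timeline, which linearly eases the Door component's relative rotation between closed and open.
; The open or close sound plays at the actor's location on every timeline update, not once per swing.
; PowerOff also prints a debug "Hello" string.
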(event `/Game/Puzzle/Cable/BI_Power.PowerOn`
  (bind (_direction _open) (`Timeline|Timeline` :!via `PlayFromStart`)
    (:`Update`
      (`SceneComponent.K2_SetRelativeRotation` (`self.Door`) (`|EaseFunction` "Linear" _open (struct) (struct :`Yaw` -100.0)) false false)
      (`GameplayStatics.PlaySoundAtLocation` (`self.OpenSFX`) (`self.K2_GetActorLocation`) (struct) 1.0 1.0 0.0 null null null null))))

(event `/Game/Puzzle/Cable/BI_Power.PowerOff`
  (`KismetSystemLibrary.PrintString` "Hello")
  (bind (_direction _open) (`Timeline|Timeline_0` :!via `PlayFromStart`)
    (:`Update`
      (`SceneComponent.K2_SetRelativeRotation` (`self.Door`) (`|EaseFunction` "Linear" _open (struct :`Yaw` -100.0)) false false)
      (`GameplayStatics.PlaySoundAtLocation` (`self.CloseSFX`) (`self.K2_GetActorLocation`) (struct) 1.0 1.0 0.0 null null null null))))

(fn `UserConstructionScript`)