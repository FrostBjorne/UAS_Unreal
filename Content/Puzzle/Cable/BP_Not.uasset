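; BP_Not is a NOT gate for the cable puzzle, controlling whether its LinkedCable fills.
; On Poweron, it sets the cable's IsFilling to the inverse of Plate1's Pressed state, after checking that the cable is valid.
; On PowerOff, it always sets IsFilling to true, without checking the plate or the cable's validity.
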(event `self.PowerOn`
  (bind _linked_cable (`self.Linked Cable`))
  (if (not (`/Game/Puzzle/Cable/BP_PressurePlateNot.pressed` (`self.Plate1`)))
    (`/Engine/EditorBlueprintResources/StandardMacros.IsValid` _linked_cable
      (:`Is Valid`
        (set `/Game/Puzzle/Cable/BP_Cable.isFilling` true _linked_cable)))
    (else
      (`/Engine/EditorBlueprintResources/StandardMacros.IsValid` _linked_cable
        (:`Is Valid`
          (set `/Game/Puzzle/Cable/BP_Cable.isFilling` false _linked_cable))))))

(event `self.PowerOff`
  (set `/Game/Puzzle/Cable/BP_Cable.isFilling` true (`self.Linked Cable`)))

(fn `UserConstructionScript`)