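; BP_PressurePlate2 is a puzzle pressure plate that powers a linked cable while something overlaps its box.
; Begin overlap plays a timeline that moves the mesh in Z, turns it blue, starts the cable filling and plays a sound.
; End overlap reverses a second timeline, turns the mesh orange and stops filling.
; Material, cable state and sound run on every timeline update, with Pressed and sound only when the cable is valid.
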(event `self.Box.OnComponentBeginOverlap`
  (params (OverlappedComponent :type "PrimitiveComponent Object Reference") (OtherActor :type "Actor Object Reference") (OtherComp :type "PrimitiveComponent Object Reference") (OtherBodyIndex :type Integer) (bFromSweep :type Boolean) (SweepResult :type "HitResult Structure (by ref)"))
  (bind _linkedcable (`self.LinkedCable`))
  ;[1 1 1] PowerOn
  (bind (_direction _newtrack_1) (`Timeline|Timeline`)
    (:`Update`
      (`SceneComponent.K2_SetRelativeLocation` (`self.StaticMesh`) (`KismetMathLibrary.MakeVector` 0.0 0.0 _newtrack_1) false false)
      (`PrimitiveComponent.SetMaterial` (`self.StaticMesh`) 0 "/Game/Puzzle/Cable/M_PrototypeGridBlue.M_PrototypeGridBlue")
      (`/Engine/EditorBlueprintResources/StandardMacros.IsValid` _linkedcable
        (:`Is Valid`
          (set `/Game/Puzzle/Cable/BP_Cable.isFilling` true _linkedcable)
          (set `self.pressed` true)
          (`GameplayStatics.PlaySoundAtLocation` (`self.ActivateSFX`) (`self.K2_GetActorLocation`) (struct) 1.0 1.0 0.0 null null null null))))))

(event `self.Box.OnComponentEndOverlap`
  (params (OverlappedComponent :type "PrimitiveComponent Object Reference") (OtherActor :type "Actor Object Reference") (OtherComp :type "PrimitiveComponent Object Reference") (OtherBodyIndex :type Integer))
  (bind _linkedcable (`self.LinkedCable`))
  ;[1 1 1] PowerOff
  (bind (_direction _newtrack_1) (`Timeline|Timeline_0` :!via `Reverse`)
    (:`Update`
      (`SceneComponent.K2_SetRelativeLocation` (`self.StaticMesh`) (`KismetMathLibrary.MakeVector` 0.0 0.0 _newtrack_1) false false)
      (`PrimitiveComponent.SetMaterial` (`self.StaticMesh`) 0 "/Game/Puzzle/Cable/M_PrototypeGridOrange.M_PrototypeGridOrange")
      (`/Engine/EditorBlueprintResources/StandardMacros.IsValid` _linkedcable
        (:`Is Valid`
          (set `/Game/Puzzle/Cable/BP_Cable.isFilling` false _linkedcable)
          (set `self.pressed` false))))))

(fn `UserConstructionScript`)