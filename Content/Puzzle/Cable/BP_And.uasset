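; BP_And is a puzzle logic gate that lets its linked cable fill only while two plates are both pressed.
; On power-on it checks both plates and sets the valid linked cable's filling flag accordingly.
; On power-off it clears that flag directly, without a validity check on the cable.
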(event `/Game/Puzzle/Cable/BI_Power.PowerOn`
  (bind _linked_cable (`self.Linked Cable`))
  (if (and (`/Game/Puzzle/Cable/BP_PressurePlate2.pressed` (`self.Plate1`)) (`/Game/Puzzle/Cable/BP_Or.pressed` (`self.Plate2`)))
    (`/Engine/EditorBlueprintResources/StandardMacros.IsValid` _linked_cable
      (:`Is Valid`
        (set `/Game/Puzzle/Cable/BP_Cable.isFilling` true _linked_cable)))
    (else
      (`/Engine/EditorBlueprintResources/StandardMacros.IsValid` _linked_cable
        (:`Is Valid`
          (set `/Game/Puzzle/Cable/BP_Cable.isFilling` false _linked_cable))))))

(event `/Game/Puzzle/Cable/BI_Power.PowerOff`
  (set `/Game/Puzzle/Cable/BP_Cable.isFilling` false (`self.Linked Cable`)))

(fn `UserConstructionScript`)