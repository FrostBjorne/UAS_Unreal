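; Puzzle 2 door actor that swings open and closed around its yaw axis.
; BeginPlay stores the SMDoor mesh's world rotation as the default.
; OpenDoor plays a timeline whose ZAxis value is combined with that stored rotation and applied to the mesh each update.
; Closedoor reverses the same timeline to swing the door back.
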(event `self.ReceiveTick`
  (params (DeltaSeconds :type "Float (single-precision)")))

(event `self.ReceiveBeginPlay`
  (set `self.Defalt Rotation` (`SceneComponent.K2_GetComponentRotation` (`self.SM_Door`))))

(event `Open Door`
  (bind (_direction _z_axis) (`Timeline|Timeline` :!label _label)
    (:`Update`
      (`SceneComponent.K2_SetWorldRotation` (`self.SM_Door`) (`KismetMathLibrary.ComposeRotators` (`KismetMathLibrary.MakeRotator` 0.0 0.0 _z_axis) (`self.Defalt Rotation`)) false false))))

(event `Close door`
  (goto _label :!via `Reverse`))

(fn `UserConstructionScript`)