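; BP_Loot_Table2 is an actor that, on BeginPlay, randomly spawns one pair of wall actors from ice, lava and slime types.
; ChooseLoot makes a weighted pick from the LootTable map by subtracting weights from a random roll up to ValueSum.
; The chosen key selects one of three pairs, spawned at the transforms of the first two Target actors.
; CalculateSum totals the weights, but Drop_Loot does not store its result in ValueSum.
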(event `self.ReceiveBeginPlay`
  (`self.Drop_Loot`))

(event `Drop_Loot`
  (`self.Calculate Sum`)
  (bind _loot (`self.Choose Loot`))
  (bind _returnvalue (`KismetStringLibrary.Conv_StringToInt` _loot))
  (if (== _returnvalue 0)
    (bind _returnvalue_2 (`|SpawnActorFromClass` "/Game/ThirdPerson/Blueprints/Morph_animation/BP_IceWall.BP_IceWall_C" (`self.GetTransform` (`|GetArrayItem` (`self.Target`))) "AlwaysSpawn" "MultiplyWithRoot" null null))
    (`|SpawnActorFromClass` "/Game/ThirdPerson/Blueprints/Morph_animation/BP_Lavawall.BP_Lavawall_C" (`self.GetTransform` (`|GetArrayItem` (`self.Target`) 1)) "AlwaysSpawn" "MultiplyWithRoot" null null)
    (elif (== _returnvalue 1)
      (`|SpawnActorFromClass` "/Game/ThirdPerson/Blueprints/Morph_animation/BP_IceWall.BP_IceWall_C" (`self.GetTransform` (`|GetArrayItem` (`self.Target`))) "AlwaysSpawn" "MultiplyWithRoot" null null)
      (`|SpawnActorFromClass` "/Game/ThirdPerson/Blueprints/Morph_animation/BP_SlimeWall.BP_SlimeWall_C" (`self.GetTransform` (`|GetArrayItem` (`self.Target`) 1)) "AlwaysSpawn" "MultiplyWithRoot" null null)
      (elif (== _returnvalue 2)
        (`|SpawnActorFromClass` "/Game/ThirdPerson/Blueprints/Morph_animation/BP_SlimeWall.BP_SlimeWall_C" (`self.GetTransform` (`|GetArrayItem` (`self.Target`))) "AlwaysSpawn" "MultiplyWithRoot" null null)
        (`|SpawnActorFromClass` "/Game/ThirdPerson/Blueprints/Morph_animation/BP_Lavawall.BP_Lavawall_C" (`self.GetTransform` (`|GetArrayItem` (`self.Target`) 1)) "AlwaysSpawn" "MultiplyWithRoot" null null)))))

(fn `Calculate Sum`
  (returns (`Total sum` :type "Float (double-precision)"))
  (locals (`Running  Total` :type "Float (double-precision)"))
  (bind _values (`BlueprintMapLibrary.Map_Values` (`self.LootTable`)))
  (for _array_element _values
    (set `local.Running  Total` (+ (`local.Running  Total`) _array_element)))
  (return (`local.Running  Total`)))

(fn `Choose Loot`
  (returns (Loot :type String))
  (locals (`Random value` :type "Float (double-precision)" :default 0.0))
  (set `local.Random value` (`KismetMathLibrary.RandomFloatInRange` 0.0 (`self.Value Sum`)))
  (bind _keys (`BlueprintMapLibrary.Map_Keys` (`self.LootTable`)))
  (for _array_element _keys
    (bind _value (`BlueprintMapLibrary.Map_Find` (`self.LootTable`) _array_element))
    (if (< (`local.Random value`) _value)
      (return _array_element)
      (else
        (set `local.Random value` (- (`local.Random value`) _value))))))

(fn `UserConstructionScript`)