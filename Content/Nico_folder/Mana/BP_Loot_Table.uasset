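; Loot table actor that, on BeginPlay, spawns fire, ice and earth books at the transforms of three Target actors.
; CalculateSum totals the LootTable map's values, and ChooseLoot uses that total for a weighted random pick of a key.
; The picked key, as 0, 1 or 2, selects one of three rotated arrangements, so the weights decide book placement while all three books are always attempted.
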(event `self.ReceiveBeginPlay`
  (`self.Drop_Loot`))

(event `Drop_Loot`
  (bind _total_sum (`self.Calculate Sum`))
  (bind _output_get (set `self.Value Sum` _total_sum))
  (`KismetSystemLibrary.PrintString` (`KismetStringLibrary.Conv_DoubleToString` _output_get))
  (bind _loot (`self.Choose Loot`))
  (bind _returnvalue (`KismetStringLibrary.Conv_StringToInt` _loot))
  (if (== _returnvalue 0)
    (bind _returnvalue_2 (`|SpawnActorFromClass` "/Game/ThirdPerson/Blueprints/Elements/Fire_book/BP_Firebook.BP_Firebook_C" (`self.GetTransform` (`|GetArrayItem` (`self.Target`))) "AdjustIfPossibleButDontSpawnIfColliding" "MultiplyWithRoot" null null))
    (`|SpawnActorFromClass` "/Game/ThirdPerson/Blueprints/Elements/Ice_Book/BP_Icebook.BP_Icebook_C" (`self.GetTransform` (`|GetArrayItem` (`self.Target`) 1)) "AdjustIfPossibleButDontSpawnIfColliding" "MultiplyWithRoot" null null)
    (`|SpawnActorFromClass` "/Game/ThirdPerson/Blueprints/Elements/Earth_book/BP_Earthbook.BP_Earthbook_C" (`self.GetTransform` (`|GetArrayItem` (`self.Target`) 2)) "AdjustIfPossibleButDontSpawnIfColliding" "MultiplyWithRoot" null null)
    (elif (== _returnvalue 1)
      (`|SpawnActorFromClass` "/Game/ThirdPerson/Blueprints/Elements/Ice_Book/BP_Icebook.BP_Icebook_C" (`self.GetTransform` (`|GetArrayItem` (`self.Target`))) "AdjustIfPossibleButDontSpawnIfColliding" "MultiplyWithRoot" null null)
      (`|SpawnActorFromClass` "/Game/ThirdPerson/Blueprints/Elements/Earth_book/BP_Earthbook.BP_Earthbook_C" (`self.GetTransform` (`|GetArrayItem` (`self.Target`) 1)) "AdjustIfPossibleButDontSpawnIfColliding" "MultiplyWithRoot" null null)
      (`|SpawnActorFromClass` "/Game/ThirdPerson/Blueprints/Elements/Fire_book/BP_Firebook.BP_Firebook_C" (`self.GetTransform` (`|GetArrayItem` (`self.Target`) 2)) "AdjustIfPossibleButDontSpawnIfColliding" "MultiplyWithRoot" null null)
      (elif (== _returnvalue 2)
        (`|SpawnActorFromClass` "/Game/ThirdPerson/Blueprints/Elements/Earth_book/BP_Earthbook.BP_Earthbook_C" (`self.GetTransform` (`|GetArrayItem` (`self.Target`))) "AdjustIfPossibleButDontSpawnIfColliding" "MultiplyWithRoot" null null)
        (`|SpawnActorFromClass` "/Game/ThirdPerson/Blueprints/Elements/Fire_book/BP_Firebook.BP_Firebook_C" (`self.GetTransform` (`|GetArrayItem` (`self.Target`) 1)) "AdjustIfPossibleButDontSpawnIfColliding" "MultiplyWithRoot" null null)
        (`|SpawnActorFromClass` "/Game/ThirdPerson/Blueprints/Elements/Ice_Book/BP_Icebook.BP_Icebook_C" (`self.GetTransform` (`|GetArrayItem` (`self.Target`) 2)) "AdjustIfPossibleButDontSpawnIfColliding" "MultiplyWithRoot" null null)))))

(fn `Calculate Sum`
  (returns (`Total sum` :type "Float (double-precision)"))
  (locals (`Running  Total` :type "Float (double-precision)"))
  (bind _values (`BlueprintMapLibrary.Map_Values` (`self.LootTable`)))
  (for _array_element _values
    (set `local.Running  Total` (+ (`local.Running  Total`) _array_element)))
  (return (`local.Running  Total`)))

(fn `Choose Loot`
  (returns (Loot :type String))
  (locals (`Random value` :type "Float (double-precision)" :default 0.0))
  (set `local.Random value` (`KismetMathLibrary.RandomFloatInRange` 0.0 (`self.Value Sum`)))
  (bind _keys (`BlueprintMapLibrary.Map_Keys` (`self.LootTable`)))
  (for _array_element _keys
    (bind _value (`BlueprintMapLibrary.Map_Find` (`self.LootTable`) _array_element))
    (if (< (`local.Random value`) _value)
      (return _array_element)
      (else
        (set `local.Random value` (- (`local.Random value`) _value))))))

(fn `UserConstructionScript`)