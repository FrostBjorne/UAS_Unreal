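; Door Blueprint that moves open or closed based on how many pressure switches are active.
; Switch activated and deactivated events raise or lower an active count, which is compared against the required number.
; Meeting the requirement plays the DoorActivate timeline and falling short reverses it, with the timeline track driving the Door component's relative Z position.
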(event `Swicth activated`
  (`/Engine/EditorBlueprintResources/StandardMacros.IncrementInt` (`self.Pressuer swicth active`)
    (:`  `
      (if (>= (`self.Pressuer swicth active`) (`self.Pressuer swicth needed`))
        (bind (_direction _door_postion) (`Timeline|Door activate` :!label _label)
          (:`Update`
            (`SceneComponent.K2_SetRelativeLocation` (`self.Door`) (`KismetMathLibrary.MakeVector` 0.0 0.0 _door_postion) false false)))
        (else
          (goto _label :!via `Reverse`))))))

(event `swicth deactivated`
  (`/Engine/EditorBlueprintResources/StandardMacros.DecrementInt` (`self.Pressuer swicth active`)
    (:`  `
      (if (>= (`self.Pressuer swicth active`) (`self.Pressuer swicth needed`))
        (goto _label)
        (else
          (goto _label :!via `Reverse`))))))

(fn `UserConstructionScript`)