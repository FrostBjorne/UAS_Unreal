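; Switch actor for a lava puzzle that triggers platforms, lava and a portal when any actor overlaps it.
; The overlap calls SwicthActivated on the referenced X, X2, Y and Y2 platforms, the lava and the portal.
; It then plays the Slip_activate timeline to slide the switch component along its relative Z axis.
; The overlap has no actor filter or once-only guard, and nothing reverses it when the overlap ends.
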(event `self.ReceiveActorBeginOverlap`
  (params (OtherActor :type "Actor Object Reference"))
  (`/Game/Nico_folder/Puzzle_2/BP_1Platform_X.Swicth activated` (`self.X_Platform`))
  (`/Game/Nico_folder/Puzzle_2/BP_Lava_Floor2.Swicth_activated` (`self.Lava to activate`))
  (`/Game/Nico_folder/Puzzle_2/BP_1Platform_Y.Swicth activated` (`self.Y_Plateform`))
  (`/Game/Nico_folder/Puzzle_2/BP_1Platform_Y2.Swicth activated` (`self.Y2_Platform`))
  (`/Game/Nico_folder/Puzzle_2/BP_1Platform_X2.Swicth activated` (`self.X2_Platform`))
  (`/Game/Nico_folder/Puzzle_1/Teleport/BP_Portal.Swicth activated` (`self.Portal`))
  (bind (_direction _swicth_position) (`Timeline|Slip_activate`)
    (:`Update`
      (`SceneComponent.K2_SetRelativeLocation` (`self.Swicth`) (`KismetMathLibrary.MakeVector` 0.0 0.0 _swicth_position) false false))))

(event `self.ReceiveActorEndOverlap`
  (params (OtherActor :type "Actor Object Reference")))

(fn `UserConstructionScript`)