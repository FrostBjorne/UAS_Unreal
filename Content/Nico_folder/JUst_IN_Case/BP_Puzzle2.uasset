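; BP_Puzzle2 is a combination puzzle actor that opens a linked door when three rotatable components match a stored code.
; An interact event rotates the given component's pitch by a set step in either direction, then checks the code.
; The check compares that component's pitch to its code entry within a small tolerance and stores the result.
; The door opens when every stored result is true and closes otherwise.
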(event `self.Interact with puzzles`
  (params (Componant :type "PrimitiveComponent Object Reference") (`Rotate Left` :type Boolean))
  (`self.Rotate` Componant `Rotate Left`))

(fn `Check Code`
  (params (Component :type "PrimitiveComponent Object Reference"))
  (locals (`Local Fail` :type Boolean) (`Select Mesh` :type Integer))
  (bind _door (`self.Door`))
  (bind (_relativerotation_roll _relativerotation_pitch) (`KismetMathLibrary.BreakRotator` (`SceneComponent.RelativeRotation` Component)))
  (if (== Component (`self.C1`))
    (set `local.Select Mesh` 0)
    (`KismetArrayLibrary.Array_Set` (`self.Code is good`) (`local.Select Mesh`) (`KismetMathLibrary.NearlyEqual_FloatFloat` (`|GetArrayItem` (`self.Code`) (`local.Select Mesh`)) _relativerotation_pitch 1.0) :!label _label)
    (for _array_element (`self.Code is good`)
      (if (not _array_element)
        (set `local.Local Fail` true)
        (break)))
    (if (`local.Local Fail`)
      (`/Game/Nico_folder/Puzzle_1/BP_Door_Puzzle2.Close door` _door)
      (else
        (`/Game/Nico_folder/Puzzle_1/BP_Door_Puzzle2.Open Door` _door)))
    (elif (== Component (`self.C2`))
      (set `local.Select Mesh` 1)
      (goto _label)
      (elif (== Component (`self.C3`))
        (set `local.Select Mesh` 2)
        (goto _label)))))

(fn `Rotate`
  (params (Comonent :type "PrimitiveComponent Object Reference") (`Rotat Left` :type Boolean))
  (if `Rotat Left`
    (`SceneComponent.K2_AddRelativeRotation` Comonent (`KismetMathLibrary.MakeRotator` 0.0 (* (`self.Rotate Value`) -1.0)) false false)
    (else
      (`SceneComponent.K2_AddRelativeRotation` Comonent (`KismetMathLibrary.MakeRotator` 0.0 (`self.Rotate Value`)) false false)
      (`KismetSystemLibrary.PrintString` (`KismetStringLibrary.Conv_RotatorToString` (`SceneComponent.RelativeRotation` Comonent)))))
  (`self.Check Code` Comonent))

(fn `UserConstructionScript`)