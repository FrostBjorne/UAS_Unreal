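; BP_CustomPadManager is a puzzle manager that opens two walls, OpenWall and OpenEnemyWall, once every tracked pad is at color index zero.
; Each Tick it loops over the pad array NewVar and clears the Finalcheck flag if any IndexColor is nonzero.
; It polls with no latch, so both open calls repeat every frame while the condition holds, including when the array is empty.
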(event `self.ReceiveTick`
  (params (DeltaSeconds :type "Float (single-precision)"))
  (set `self.finalcheck` 1)
  (for _array_element (`self.NewVar`)
    (if (!= (`/Game/Gerardo_level/BP_CustomPad.indexColor` _array_element) 0)
      (set `self.finalcheck` 0)))
  (if (== (`self.finalcheck`) 1)
    (`/Game/Gerardo_level/BP_Wall.Open Wall` (`self.OpenWall`))
    (`/Game/Gerardo_level/BP_EnemyWall.Open Enemy Wall` (`self.OpenEnemyWall`))))

(fn `UserConstructionScript`)