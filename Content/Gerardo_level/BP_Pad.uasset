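; BP_Pad is a toggle pad for what appears to be a Lights Out style puzzle.
; When a BP_ThirdPersonCharacter overlaps its Box, the pad flips its own IsOn state and that of every pad in AdjacentPads.
; Tick polls IsOn to swap the Cube between on and off materials and to set an Index value matching the state.
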(event `self.ReceiveTick`
  (params (DeltaSeconds :type "Float (single-precision)"))
  (bind _cube (`self.Cube`))
  (if (`self.IsOn?`)
    (`PrimitiveComponent.SetMaterial` _cube 0 "/Game/Gerardo_level/M_IsON.M_IsON")
    (set `self.Index` 0)
    (else
      (`PrimitiveComponent.SetMaterial` _cube 0 "/Game/Gerardo_level/M_IsOff.M_IsOff")
      (set `self.Index` 1))))

(event `self.Box.OnComponentBeginOverlap`
  (params (OverlappedComponent :type "PrimitiveComponent Object Reference") (OtherActor :type "Actor Object Reference") (OtherComp :type "PrimitiveComponent Object Reference") (OtherBodyIndex :type Integer) (bFromSweep :type Boolean) (SweepResult :type "HitResult Structure (by ref)"))
  (if (== (`GameplayStatics.GetObjectClass` OtherActor) "/Game/ThirdPerson/Blueprints/BP_ThirdPersonCharacter.BP_ThirdPersonCharacter_C")
    (if (`self.IsOn?`)
      (set `self.IsOn?` false)
      (else
        (set `self.IsOn?` true)))
    (for _array_element (`self.AdjacentPads`)
      (if (`/Game/Gerardo_level/BP_Pad.IsOn?` _array_element)
        (set `/Game/Gerardo_level/BP_Pad.IsOn?` false _array_element)
        (else
          (set `/Game/Gerardo_level/BP_Pad.IsOn?` true _array_element))))))

(fn `UserConstructionScript`)