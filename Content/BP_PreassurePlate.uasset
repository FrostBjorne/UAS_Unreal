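; Pressure plate actor that detects whether its assigned statue has been placed on it, likely as part of a puzzle.
; Collision overlap plays a timeline that lerps the Plate mesh down, and end overlap reverses it.
; When the timeline finishes, IsPlateFilledCorrectly is set true if the overlapping actor is StatueRef; no live path clears it.
; Statue cast, tag check and door switch nodes are disconnected and never run.
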(event `self.Collision.OnComponentBeginOverlap`
  (params (OverlappedComponent :type "PrimitiveComponent Object Reference") (OtherActor :type "Actor Object Reference") (OtherComp :type "PrimitiveComponent Object Reference") (OtherBodyIndex :type Integer) (bFromSweep :type Boolean) (SweepResult :type "HitResult Structure (by ref)"))
  (bind (_direction _newtrack_0) (`Timeline|Plate Timeline` :!label _label)
    (:`Update`
      (`SceneComponent.K2_SetRelativeLocation` (`self.Plate`) (`KismetMathLibrary.MakeVector` 0.0 0.0 (`KismetMathLibrary.Lerp` 20.0 12.0 _newtrack_0)) false false))
    (:`Finished`
      (if (== OtherActor (`self.StatueRef`))
        (set `self.bIsPlateFilledCorrectly` true)))))

(event `self.Collision.OnComponentEndOverlap`
  (params (OverlappedComponent :type "PrimitiveComponent Object Reference") (OtherActor :type "Actor Object Reference") (OtherComp :type "PrimitiveComponent Object Reference") (OtherBodyIndex :type Integer))
  (goto _label :!via `Reverse`))

(fn `UserConstructionScript`)