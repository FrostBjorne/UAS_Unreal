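; BP_ObjectSpawner is a puzzle logic object that spawns a configured actor class above itself when it enters the Activate state.
; Spawning plays sound and particle effects and is gated by a valid class and a cooldown counted down on Tick.
; An optional one-at-a-time mode destroys the previous spawn with an effect first.
; The construction script sets up an optional preview mesh with an override material, which Tick rotates.
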(event `/Game/Puzzle2/Blueprints/Misc/BPI_PuzzleLogic.OnEnterState`
  (params (State :type "/Game/Puzzle2/Blueprints/Misc/ENUM_LogicTriggerStates Enum" :default "NewEnumerator0"))
  (bind _returnvalue (+ (`self.K2_GetActorLocation`) (`KismetMathLibrary.MakeVector` 0.0 0.0 (`self.SpawnZOffset`))))
  ;[1 1 1] Puzzle logic event received to spawn the specified actor.
  ; If the spawner is set to only allow one spawned object at a time, any previously spawned objects are destroyed.
  (`parent.OnEnterState` State)
  (switch `/Game/Puzzle2/Blueprints/Misc/ENUM_LogicTriggerStates` State
    (:`NewEnumerator0`
      (if (`self.CanSpawn`)
        (if (`self.AllowOneOnly`)
          (`/Engine/EditorBlueprintResources/StandardMacros.IsValid` (`self.SpawnedActor`)
            (:`Is Valid`
              (`GameplayStatics.SpawnEmitterAtLocation` (`self.DestroyFX`) (`self.K2_GetActorLocation` (`self.SpawnedActor`)))
              (`self.K2_DestroyActor` (`self.SpawnedActor`)))
            (:`Is Not Valid`
              _)))
        (`GameplayStatics.PlaySoundAtLocation` (`self.SpawnObjectSFX`) (`self.K2_GetActorLocation`) (struct) 1.0 1.0 0.0 null null null null)
        (bind _returnvalue_2 (`|SpawnActorFromClass` (`self.ActorToSpawn`) (`KismetMathLibrary.Conv_VectorToTransform` _returnvalue) "Undefined" "SelectDefaultAtRuntime" null null))
        (set `self.SpawnedActor` _returnvalue_2)
        (`GameplayStatics.SpawnEmitterAtLocation` (`self.SpawnFX`) _returnvalue)
        (set `self.SpawnCooldownRemaining` (`self.SpawnCooldown`))))))

(event `self.ReceiveTick`
  (params (DeltaSeconds :type "Float (single-precision)"))
  ;[1 1 1] Update cooldown, and rotate the visual preview mesh.
  (`parent.ReceiveTick` DeltaSeconds)
  (`|ExecutionSequence`
    (:`then_0`
      (if (> (`self.SpawnCooldownRemaining`) 0.0)
        (set `self.SpawnCooldownRemaining` (- (`self.SpawnCooldownRemaining`) DeltaSeconds))))
    (:`then_1`
      (if (`self.ShowPreviewMesh`)
        (`SceneComponent.K2_AddWorldRotation` (`self.PreviewStaticMesh`) (`KismetMathLibrary.MakeRotator` 0.0 0.0 (* DeltaSeconds (`self.PreviewMeshRotateSpeed`))) false true)))))

(fn `CanSpawn`
  (returns (Success :type Boolean))
  ;[1 1 1] Checks there is a valid input actor type to spawn, and the spawner is not currently on cooldown.
  (if (`KismetSystemLibrary.IsValidClass` (`self.ActorToSpawn`))
    (if (<= (`self.SpawnCooldownRemaining`) 0.0)
      (return true)
      (else
        _))
    (else
      (`KismetSystemLibrary.PrintString` "No spawn actor set")))
  (return false))

(fn `UserConstructionScript`
  (bind _previewmesh (`self.PreviewMesh`))
  (bind _previewstaticmesh (`self.PreviewStaticMesh`))
  ;[1 1 1] Sets the mesh of the visual preview mesh, and sets its materials to an emissive blue.
  ; OR hides the visual preview mesh it if it is set to not show.
  (`parent.UserConstructionScript`)
  (if (`self.ShowPreviewMesh`)
    (`/Engine/EditorBlueprintResources/StandardMacros.IsValid` _previewmesh
      (:`Is Valid`
        (`StaticMeshComponent.SetStaticMesh` _previewstaticmesh _previewmesh)
        (`SceneComponent.SetVisibility` _previewstaticmesh true true)
        (`SceneComponent.K2_SetRelativeTransform` _previewstaticmesh (`self.PreviewMeshTransform`) false false)
        (for (_ _array_index) (`MeshComponent.GetMaterials` _previewstaticmesh)
          (`PrimitiveComponent.SetMaterial` _previewstaticmesh _array_index "/Game/Puzzle2/Materials/M_SpawnerPreviewMesh.M_SpawnerPreviewMesh")))
      (:`Is Not Valid`
        (`SceneComponent.SetVisibility` _previewstaticmesh false true :!label _label)))
    (else
      (goto _label))))