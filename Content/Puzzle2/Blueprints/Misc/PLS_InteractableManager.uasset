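; Interactable manager that picks the one object the player can interact with and owns the on-screen interact prompt.
; Interactables add themselves when in range and angle; each Tick it drops invalid ones and picks the closest to this actor, with held physics objects taking priority.
; Input is enabled only on the chosen actor, so only it responds.
; It creates the prompt widget when missing and hides it when nothing is selected.
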(event `self.ReceiveTick`
  (params (DeltaSeconds :type "Float (single-precision)"))
  ;[1 1 1] Each frame, determine which "interactable" object is the most valid (determined by its distance and angle from the player character).
  ; If none exist, hide the interact prompt widget.
  (`/Engine/EditorBlueprintResources/StandardMacros.IsValid` (`self.WidgetInteractPrompt`)
    (:`Is Valid`
      (`self.SetMostValidInteractActor`)
      (`/Engine/EditorBlueprintResources/StandardMacros.IsValid` (`self.MostValidInteractActor`)
        (:`Is Not Valid`
          (`self.HidePrompt`))))
    (:`Is Not Valid`
      (`self.AttemptAddInteractPrompt`))))

(fn `AddInteractableObjectInRangeAndAngle`
  (params (Actor :type "/Game/Puzzle2/Blueprints/LogicObjects/ParentClasses/BP_LogicObject_Interactable_Base Object Reference"))
  ;[1 1 1] Called by actors of type "BP_LogicObject_Interactable_Base" to add itself to this actor's valid interactable objects list.
  ; They will only attempt to add themself to the list if they are in interactable range and within a certain angle of the player's facing direction.
  (if (not (`KismetArrayLibrary.Array_Contains` (`self.ValidInteractableActors`) Actor))
    (`KismetArrayLibrary.Array_AddUnique` (`self.ValidInteractableActors`) Actor)))

(fn `AttemptAddInteractPrompt`
  (bind _returnvalue (`PlayerController.GetHUD` (`GameplayStatics.GetPlayerController` 0)))
  ;[1 1 1] Attempt to add the interact widget prompt to the screen.
  (`/Engine/EditorBlueprintResources/StandardMacros.IsValid` _returnvalue
    (:`Is Valid`
      (bind _returnvalue_2 (`AddComponent|NODE_AddWidgetComponent-0` :`self` _returnvalue))
      (bind _returnvalue_3 (`|CreateWidget` "/Game/Puzzle2/UI/Widget_InteractPrompt.Widget_InteractPrompt_C" (`GameplayStatics.GetPlayerController` 0)))
      (bind _output_get (set `self.WidgetInteractPrompt` _returnvalue_3))
      (`WidgetComponent.SetWidget` _returnvalue_2 _output_get)
      (`UserWidget.AddToPlayerScreen` _returnvalue_3 0)
      (`WidgetComponent.SetWidgetSpace` _returnvalue_2 "Screen"))
    (:`Is Not Valid`
      ;[1 1 1] Add widget directly to screen if there is no HUD
      (bind _returnvalue_4 (`|CreateWidget` "/Game/Puzzle2/UI/Widget_InteractPrompt.Widget_InteractPrompt_C" (`GameplayStatics.GetPlayerController` 0)))
      (bind _output_get_2 (set `self.WidgetInteractPrompt` _returnvalue_4))
      (`UserWidget.AddToViewport` _output_get_2 0))))

(fn `HidePrompt`
  (bind _widgetinteractprompt (`self.WidgetInteractPrompt`))
  ;[1 1 1] Hide interact prompt.
  (`/Engine/EditorBlueprintResources/StandardMacros.IsValid` _widgetinteractprompt
    (:`Is Valid`
      (`/Game/Puzzle2/UI/Widget_InteractPrompt.Hide` _widgetinteractprompt))))

(fn `SetMostValidInteractActor`
  (locals (ClosestDistance :type "Float (double-precision)" :default 100000000.0) (HeldObjectFound :type Boolean) (TempActor :type "/Game/Puzzle2/Blueprints/LogicObjects/ParentClasses/BP_LogicObject_Interactable_Base Object Reference"))
  (bind _tempactor (`local.TempActor`))
  (bind _mostvalidinteractactor (`self.MostValidInteractActor`))
  (bind _returnvalue (`KismetMathLibrary.VSize` (- (`self.K2_GetActorLocation` _tempactor) (`self.K2_GetActorLocation`))))
  (`|ExecutionSequence`
    (:`then_0`
      (set `self.MostValidInteractActor` null)
      (for _array_element (`self.ValidInteractableActors`)
        (bind _output_get (set `local.TempActor` _array_element))
        (`/Engine/EditorBlueprintResources/StandardMacros.IsValid` _array_element
          (:`Is Valid`
            ;[1 1 1] If physics object is already held, then IT IS the most valid interact object, as other objects cannot be interacted with while a physics object is being held.
            (bind _asbp_logic_object_physics_base (cast `/Game/Puzzle2/Blueprints/LogicObjects/ParentClasses/BP_LogicObject_Physics_Base` _output_get)
              (:`then`
                (if (`/Game/Puzzle2/Blueprints/LogicObjects/ParentClasses/BP_LogicObject_Physics_Base.IsHeld` _asbp_logic_object_physics_base)
                  (set `self.MostValidInteractActor` _asbp_logic_object_physics_base)
                  (set `local.HeldObjectFound` true)
                  (else
                    ;[1 1 1] If multiple actors are in a valid distance and angle to be interacted with, select the closest one.
                    ; Also check if any previously determined valid interactable object is no longer valid. If so, remove from list.
                    (if (`/Game/Puzzle2/Blueprints/LogicObjects/ParentClasses/BP_LogicObject_Interactable_Base.IsValidInteractObject` _tempactor) :!label _label
                      (if (`local.HeldObjectFound`)
                        _
                        (elif (< _returnvalue (`local.ClosestDistance`))
                          (set `self.MostValidInteractActor` (`local.TempActor`))
                          (set `local.ClosestDistance` _returnvalue)))
                      (else
                        (`self.DisableInput` (`local.TempActor`) (`GameplayStatics.GetPlayerController` 0))
                        (`KismetArrayLibrary.Array_RemoveItem` (`self.ValidInteractableActors`) (`local.TempActor`) :!label _label_2))))))
              (:`CastFailed`
                (goto _label))))
          (:`Is Not Valid`
            (goto _label_2)))))
    (:`then_1`
      ;[1 1 1] Ensure only the selected interactable object has valid input and can be interacted with.
      ; Turn off input for all others.
      (for _array_element_2 (`self.ValidInteractableActors`)
        (`self.DisableInput` _array_element_2 (`GameplayStatics.GetPlayerController` 0)))
      (`/Engine/EditorBlueprintResources/StandardMacros.IsValid` _mostvalidinteractactor
        (:`Is Valid`
          (`self.EnableInput` _mostvalidinteractactor (`GameplayStatics.GetPlayerController` 0)))))))

(fn `ShowPrompt`
  (params (Text :type Text))
  (bind _widgetinteractprompt (`self.WidgetInteractPrompt`))
  ;[1 1 1] Show interact prompt.
  (`/Engine/EditorBlueprintResources/StandardMacros.IsValid` _widgetinteractprompt
    (:`Is Valid`
      (`/Game/Puzzle2/UI/Widget_InteractPrompt.Show` _widgetinteractprompt Text))))

(fn `UserConstructionScript`)