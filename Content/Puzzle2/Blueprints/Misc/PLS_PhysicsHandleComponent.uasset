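; Physics handle wrapper that lets the player pick up, carry and drop physics objects.
; GrabObject attaches a component to the PhysicsHandle, and Tick targets it at a set distance and height offset from the pawn, along camera or pawn forward, facing that direction.
; Pickups are smoothed by dropping interpolation speed on grab, then lerping it back to the default cached in the construction script.
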(event `self.ReceiveTick`
  (params (DeltaSeconds :type "Float (single-precision)"))
  ;[1 1 1] Update the position of the physics object.
  (`/Engine/EditorBlueprintResources/StandardMacros.IsValid` (`self.HoldObject`)
    (:`Is Valid`
      (`self.UpdatePhysicsObjectLocation`)
      (`self.UpdateInterpolationSpeed`))))

(fn `DropObject`
  ;[1 1 1] Remove the object held on the physics handle component.
  (`PhysicsHandleComponent.ReleaseComponent` (`self.PhysicsHandle`))
  (set `self.HoldObject` null))

(fn `GrabObject`
  (params (Component1 :type "PrimitiveComponent Object Reference") (ActorHeld :type "Actor Object Reference") (DistanceToHoldObjectInFront :type "Float (double-precision)"))
  ;[1 1 1] Assign the object held on the physics handle component.
  ; Set the interpolation speed (the speed of the object to pick up moving from sitting on the ground to beind held in front) to a slow value, and let it build up over time.
  ; This smooths out the "pick up object" transition.
  (set `self.DistanceInFront` DistanceToHoldObjectInFront)
  (set `self.HoldObject` ActorHeld)
  (`PhysicsHandleComponent.GrabComponentAtLocationWithRotation` (`self.PhysicsHandle`) Component1 "None" (`SceneComponent.K2_GetComponentLocation` Component1) (`SceneComponent.K2_GetComponentRotation` Component1))
  (`PhysicsHandleComponent.SetInterpolationSpeed` (`self.PhysicsHandle`) 2.0)
  (set `self.IsIncreasingInterpSpeed` true))

(fn `UpdateInterpolationSpeed`
  (locals (NewLerpedValue :type "Float (double-precision)"))
  (bind _newlerpedvalue (`local.NewLerpedValue`))
  (bind _physicshandle (`self.PhysicsHandle`))
  ;[1 1 1] Build up the speed of "picking up the object" over time.
  ; This makes picking up objects appear smoother.
  (if (`self.IsIncreasingInterpSpeed`)
    (set `local.NewLerpedValue` (`KismetMathLibrary.Lerp` (`PhysicsHandleComponent.InterpolationSpeed` (`self.PhysicsHandle`)) (`self.StartingInterpolationSpeed`) (* (`GameplayStatics.GetWorldDeltaSeconds`) 1.0)))
    (if (> _newlerpedvalue (- (`self.StartingInterpolationSpeed`) 10.0))
      (`PhysicsHandleComponent.SetInterpolationSpeed` _physicshandle (`self.StartingInterpolationSpeed`))
      (set `self.IsIncreasingInterpSpeed` false)
      (else
        (`PhysicsHandleComponent.SetInterpolationSpeed` _physicshandle _newlerpedvalue)))))

(fn `UpdatePhysicsObjectLocation`
  (locals (ObjectPositionInFront :type "Vector Structure" :default (0.0 0.0 0.0)))
  (bind _physicshandle (`self.PhysicsHandle`))
  ;[1 1 1] This sets the object held to a specific distance in front of the player character.
  (if (`self.UsePlayerForwardInsteadOfCamera`)
    (set `local.ObjectPositionInFront` (* (`self.GetActorForwardVector` (`GameplayStatics.GetPlayerPawn` 0)) (`self.DistanceInFront`)))
    (else
      (bind _output_get (set `local.ObjectPositionInFront` (* (`KismetMathLibrary.GetForwardVector` (`PlayerCameraManager.GetCameraRotation` (`GameplayStatics.GetPlayerCameraManager` 0))) (`self.DistanceInFront`))))))
  (`PhysicsHandleComponent.SetTargetLocation` _physicshandle (+ _output_get (+ (`self.K2_GetActorLocation` (`GameplayStatics.GetPlayerPawn` 0)) (`KismetMathLibrary.MakeVector` 0.0 0.0 (`self.DistanceHeightOffset`)))))
  (`PhysicsHandleComponent.SetTargetRotation` _physicshandle (`KismetMathLibrary.Conv_VectorToRotator` (`local.ObjectPositionInFront`))))

(fn `UserConstructionScript`
  ;[1 1 1] Set the starting interpolation speed, taken from the default physics handle value.
  (set `self.StartingInterpolationSpeed` (`PhysicsHandleComponent.InterpolationSpeed` (`self.PhysicsHandle`))))