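; BP_PuzzleLogicVisualiser is an editor debug actor that draws lines showing how puzzle logic objects are wired together.
; When ShowLines is on, its construction script finds every BP_LogicObject_Base and draws long-lived debug lines to actors linked in each of its trigger-state arrays.
; The lines are flushed before each redraw or when ShowLines is off.
; BeginPlay sets ShowLines to false to keep the lines out of gameplay.
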(event `self.ReceiveBeginPlay`
  ;[1 1 1] Turn off debug lines so they don't show when the game starts.
  (`parent.ReceiveBeginPlay`)
  (set `self.ShowLines` false))

(fn `DrawDebugLinesForActor`
  (params (Actor :type "/Game/Puzzle2/Blueprints/LogicObjects/ParentClasses/BP_LogicObject_Base Object Reference"))
  (locals (Actor_Local :type "/Game/Puzzle2/Blueprints/LogicObjects/ParentClasses/BP_LogicObject_Base Object Reference"))
  (bind _actor_local (`local.Actor_Local`))
  (bind _actor_local_2 (`local.Actor_Local`))
  (bind _actor_local_3 (`local.Actor_Local`))
  (bind _actor_local_4 (`local.Actor_Local`))
  (bind _actor_local_5 (`local.Actor_Local`))
  (bind _actor_local_6 (`local.Actor_Local`))
  ;[1 1 1] For each puzzle logic actor, drawn connections between itself and any actors linked to ANY of its trigger states.
  (set `local.Actor_Local` Actor)
  (`|ExecutionSequence`
    (:`then_0`
      (`self.DrawLinesSegments` _actor_local_6 (`/Game/Puzzle2/Blueprints/LogicObjects/ParentClasses/BP_LogicObject_Base.OnActivated` _actor_local_6))
      (`self.DrawLinesSegments` _actor_local_6 (`/Game/Puzzle2/Blueprints/LogicObjects/ParentClasses/BP_LogicObject_Base.OnDeactivated` _actor_local_6))
      (`self.DrawLinesSegments` _actor_local_2 (`/Game/Puzzle2/Blueprints/LogicObjects/ParentClasses/BP_LogicObject_Base.OnPaused` _actor_local_2))
      (`self.DrawLinesSegments` _actor_local_2 (`/Game/Puzzle2/Blueprints/LogicObjects/ParentClasses/BP_LogicObject_Base.OnInteractable` _actor_local_2)))
    (:`then_1`
      (`self.DrawLinesSegments` _actor_local_3 (`/Game/Puzzle2/Blueprints/LogicObjects/ParentClasses/BP_LogicObject_Base.OnUninteractable` _actor_local_3))
      (`self.DrawLinesSegments` _actor_local_3 (`/Game/Puzzle2/Blueprints/LogicObjects/ParentClasses/BP_LogicObject_Base.OnState1` _actor_local_3))
      (`self.DrawLinesSegments` _actor_local_4 (`/Game/Puzzle2/Blueprints/LogicObjects/ParentClasses/BP_LogicObject_Base.OnState2` _actor_local_4))
      (`self.DrawLinesSegments` _actor_local_4 (`/Game/Puzzle2/Blueprints/LogicObjects/ParentClasses/BP_LogicObject_Base.OnState3` _actor_local_4)))
    (:`then_2`
      (`self.DrawLinesSegments` _actor_local_5 (`/Game/Puzzle2/Blueprints/LogicObjects/ParentClasses/BP_LogicObject_Base.OnState4` _actor_local_5))
      (`self.DrawLinesSegments` _actor_local_5 (`/Game/Puzzle2/Blueprints/LogicObjects/ParentClasses/BP_LogicObject_Base.OnState5` _actor_local_5))
      (`self.DrawLinesSegments` _actor_local (`/Game/Puzzle2/Blueprints/LogicObjects/ParentClasses/BP_LogicObject_Base.OnDisabled` _actor_local)))))

(fn `DrawLinesSegments`
  (params (ParentActor :type "/Game/Puzzle2/Blueprints/LogicObjects/ParentClasses/BP_LogicObject_Base Object Reference") (TriggerObjects :type "Array of /Game/Puzzle2/Blueprints/Misc/STRUCT_LogicTriggerActor Structure"))
  (locals (Offset :type "Vector Structure" :default (0.0 0.0 10.0)))
  ;[1 1 1] Actual logic to draw line between puzzle logic actor and linked actor.
  (for _array_element TriggerObjects
    (bind _actortotrigger (break `/Game/Puzzle2/Blueprints/Misc/STRUCT_LogicTriggerActor` _array_element))
    (`/Engine/EditorBlueprintResources/StandardMacros.IsValid` _actortotrigger
      (:`Is Valid`
        (`KismetSystemLibrary.DrawDebugLine` (+ (`self.K2_GetActorLocation` ParentActor) (`local.Offset`)) (+ (`self.K2_GetActorLocation` _actortotrigger) (`local.Offset`)) (struct :`R` 0.473958 :`G` 0.301838 :`B` 0.012798 :`A` 1.0) 99999997952.0 10.0)))))

(fn `UpdateConnections`
  ;[1 1 1] Clear all lines from last update and re-draw connections between all puzzle logic actors.
  (if (`self.ShowLines`)
    (`KismetSystemLibrary.FlushPersistentDebugLines`)
    (bind _outactors (`GameplayStatics.GetAllActorsOfClass` "/Game/Puzzle2/Blueprints/LogicObjects/ParentClasses/BP_LogicObject_Base.BP_LogicObject_Base_C"))
    (for _array_element _outactors
      (`self.DrawDebugLinesForActor` _array_element))))

(fn `UserConstructionScript`
  ;[1 1 1] Update all connections between puzzle logic actors.
  (if (`self.ShowLines`)
    (`self.UpdateConnections`)
    (else
      (`KismetSystemLibrary.FlushPersistentDebugLines`))))